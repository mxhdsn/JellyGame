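; Door Blueprint with two hinged leaves that swing open when the first-person character enters its trigger box.
; On overlap it stores the player and, if it can open and is not already open, hides the NoEntry component and plays the Open timeline.
; The timeline's two tracks rotate the left and right pivots outward in opposite yaw directions; there is no closing logic.
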(event OnComponentBeginOverlap(Box)
  (params (OverlappedComponent :type Primitive%20Component%20Object%20Reference) (OtherActor :type Actor%20Object%20Reference) (OtherComp :type Primitive%20Component%20Object%20Reference) (OtherBodyIndex :type Integer) (bFromSweep :type Boolean) (SweepResult :type Hit%20Result%20Structure%20%28by%20ref%29))
  (bind _asbp_first_person_character (Utilities|Casting|CastToBP_FirstPersonCharacter OtherActor))
  (Variables|Default|SetPlayer _asbp_first_person_character)
  (if (and (Variables|Default|GetCanOpen?) (Variables|Default|GetNotOpened))
    (Variables|Default|SetDoorOpen true)
    (Development|SetHiddeninGame (Variables|Default|GetNoEntry) true false)
    (bind (_direction _doorleft _doorright) (Timeline|Open Play)
      (:Update
        (Transformation|SetRelativeRotation (Variables|Default|GetPivotLeft) (Math|Rotator|MakeRotator 0.0 0.0 (Math|Float|Lerp 0.0 -1.1e+02 _doorleft)) false false)
        (Transformation|SetRelativeRotation (Variables|Default|GetPivotRight) (Math|Rotator|MakeRotator 0.0 0.0 (Math|Float|Lerp 0.0 1.1e+02 _doorright)) false false)))))

(event EventBeginPlay)

(fn ConstructionScript)