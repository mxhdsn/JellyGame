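; Child door Blueprint that grants access once the first-person player has hit enough targets.
; On overlap it runs the parent logic, reads TargetsHit from player pawn 0, and at five or more sets CanOpen and reruns the parent overlap once.
; Below that it clears the character's AreTargetsHit and prints a one-time denial citing six targets, unlike the check.
; Leaving the Box sets AreTargetsHit true regardless of count.
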(event OnComponentEndOverlap(Box)
  (params (OverlappedComponent :type Primitive%20Component%20Object%20Reference) (OtherActor :type Actor%20Object%20Reference) (OtherComp :type Primitive%20Component%20Object%20Reference) (OtherBodyIndex :type Integer))
  (bind _asbp_first_person_character (Utilities|Casting|CastToBP_FirstPersonCharacter OtherActor))
  (Variables|/Game/FirstPerson/Blueprints/BP_FirstPersonCharacter.BP_FirstPersonCharacter_C|SetareTargetsHit _asbp_first_person_character true))

(event Collision|EventActorBeginOverlap
  (params (OtherActor :type Actor%20Object%20Reference))
  (|CallParentFunction OtherActor)
  (bind _asbp_first_person_character (Utilities|Casting|CastToBP_FirstPersonCharacter (Game|Player|GetPlayerPawn 0)))
  (Development|PrintString (Utilities|String|ToString(Integer) (Variables|/Game/FirstPerson/Blueprints/BP_FirstPersonCharacter.BP_FirstPersonCharacter_C|GetTargetsHit _asbp_first_person_character)))
  (if (>= (Variables|/Game/FirstPerson/Blueprints/BP_FirstPersonCharacter.BP_FirstPersonCharacter_C|GetTargetsHit _asbp_first_person_character) 5)
    (Utilities|FlowControl|DoOnce false
      (:Completed
        (Variables|Default|SetCanOpen? true)
        (Development|PrintString "ACCESS GRANTED")
        (|CallParentFunction OtherActor)))
    (else
      (Variables|/Game/FirstPerson/Blueprints/BP_FirstPersonCharacter.BP_FirstPersonCharacter_C|SetareTargetsHit _asbp_first_person_character false)
      (Utilities|FlowControl|DoOnce false
        (:Completed
          (Development|PrintString "ACCESS DENIED MUST HIT ALL 6 TARGETS"))))))

(event EventBeginPlay
  (Variables|Default|SetCanOpen? false))

(fn ConstructionScript
  (|CallParentFunction))