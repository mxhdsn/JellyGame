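; BP_Enemy is a jelly enemy that loses health to player bullets, damages the player on contact, and is destroyed at zero health.
; Damage arrives through projectile overlaps on its Box or through HitByBullet, which also scales the dynamic material's emissive value with remaining health.
; Player overlap starts a short timer that calls DamagePlayer on the cached character if the overlap persists.
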(event OnComponentBeginOverlap(Box)
  (params (OverlappedComponent :type Primitive%20Component%20Object%20Reference) (OtherActor :type Actor%20Object%20Reference) (OtherComp :type Primitive%20Component%20Object%20Reference) (OtherBodyIndex :type Integer) (bFromSweep :type Boolean) (SweepResult :type Hit%20Result%20Structure%20%28by%20ref%29))
  (bind _asbp_first_person_projectile (Utilities|Casting|CastToBP_FirstPersonProjectile OtherActor))
  (Variables|Default|SetHealth (- (Variables|Default|GetHealth) (Variables|/Game/FirstPerson/Blueprints/BP_FirstPersonProjectile.BP_FirstPersonProjectile_C|GetBulletDamage _asbp_first_person_projectile)))
  (if (<= (Variables|Default|GetHealth) 0)
    (Actor|DestroyActor)))

(event Custom|EnemyHitPlayer
  (if (Collision|IsOverlappingActor (Game|GetPlayerCharacter 0) :!class /Script/Engine.Actor)
    (Default|DamagePlayer (Variables|Default|GetPlayer%20Cast))))

(event Collision|EventActorBeginOverlap
  (params (OtherActor :type Actor%20Object%20Reference))
  (if (== OtherActor (Game|GetPlayerCharacter 0))
    (Utilities|Time|SetTimerbyEvent (delegate Custom|EnemyHitPlayer) 0.1)))

(event EventBeginPlay
  (bind _returnvalue (Rendering|Material|CreateDynamicMaterialInstance "/Game/Models/Enemy/Jelly_Monster/LOW_EnemieMat.LOW_EnemieMat" "None" "None" :!class /Script/Engine.KismetMaterialLibrary))
  (bind _output_get (Variables|Default|SetDynamic%20Mat%20Inst _returnvalue))
  (Rendering|Material|SetMaterial (Variables|Default|GetJelly_Enemy_LOW) 0 _output_get)
  (bind _asbp_first_person_character (Utilities|Casting|CastToBP_FirstPersonCharacter (Game|GetPlayerCharacter 0)))
  (Variables|Default|SetPlayer%20Cast _asbp_first_person_character))

(fn ConstructionScript)

(fn HitbyBullet
  (params (BulletDamage :type Integer))
  (bind _output_get (Variables|Default|SetHealth (- (Variables|Default|GetHealth) BulletDamage)))
  (Rendering|Material|SetScalarParameterValueonMaterials (Variables|Default|GetJelly_Enemy_LOW) "Dynamic Emissive  Value" (/ (Math|Conversions|ToFloat(Integer) _output_get) 4.0))
  (if (<= _output_get 0)
    (Actor|DestroyActor)))