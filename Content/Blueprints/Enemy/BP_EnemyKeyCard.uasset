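; BP_EnemyKeyCard is an enemy variant that carries a keycard and awards it to the player on death.
; BeginPlay passes itself and its KcDoor reference to the WBP_EnemyKC widget on its Keycard component.
; Tick rotates that component to face the player pawn.
; Death uses KcNum to update the keycard display in the player's main UI and give the player that keycard.
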(event EventBeginPlay
  (|CallParentFunction)
  (bind _aswbp_enemy_kc (Utilities|Casting|CastToWBP_EnemyKC (UserInterface|GetUserWidgetObject (Variables|Default|GetKeycard))))
  (Variables|/Game/Blueprints/UI/WBP_EnemyKC.WBP_EnemyKC_C|SetEnemyRef _aswbp_enemy_kc self)
  (Variables|/Game/Blueprints/UI/WBP_EnemyKC.WBP_EnemyKC_C|SetKcDoor _aswbp_enemy_kc (Variables|Default|GetKcDoor)))

(event Collision|EventActorBeginOverlap
  (params (OtherActor :type Actor%20Object%20Reference))
  (|CallParentFunction OtherActor) ; This node is disabled and will not be called.\nDrag off pins to build functionality.
)

(event EventTick
  (params (DeltaSeconds :type Float%20%28single-precision%29))
  (bind _keycard (Variables|Default|GetKeycard))
  (Transformation|SetWorldRotation _keycard (Math|Rotator|FindLookatRotation (Transformation|GetWorldLocation _keycard) (Transformation|GetActorLocation (Game|Player|GetPlayerPawn 0))) false false))

(event EventDeath
  (bind _player_cast (Variables|Default|GetPlayer%20Cast))
  (bind _kc_num (Variables|Default|GetKc_Num))
  (Default|SetKcVis (Variables|/Game/FirstPerson/Blueprints/BP_FirstPersonCharacter.BP_FirstPersonCharacter_C|GetMainUI _player_cast) _kc_num)
  (Default|GetKeyCard _player_cast _kc_num))

(fn ConstructionScript
  (|CallParentFunction))