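; Boss enemy actor that loses health when hit by player bullets and destroys itself once health runs out.
; Damage arrives either through a collision box overlap with a first-person projectile or through the HitByBullet function, which also prints remaining health.
; The two paths end differently: an overlap kill sets IsBossDead on the player character, while a HitByBullet kill calls the character's WinGame.
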(event OnComponentBeginOverlap(CollisionBox)
  (params (OverlappedComponent :type Primitive%20Component%20Object%20Reference) (OtherActor :type Actor%20Object%20Reference) (OtherComp :type Primitive%20Component%20Object%20Reference) (OtherBodyIndex :type Integer) (bFromSweep :type Boolean) (SweepResult :type Hit%20Result%20Structure%20%28by%20ref%29))
  (bind _asbp_first_person_projectile (Utilities|Casting|CastToBP_FirstPersonProjectile OtherActor))
  (Variables|Default|SetBossHealth (- (Variables|Default|GetBossHealth) (Variables|/Game/FirstPerson/Blueprints/BP_FirstPersonProjectile.BP_FirstPersonProjectile_C|GetBulletDamage _asbp_first_person_projectile)))
  (if (<= (Variables|Default|GetBossHealth) 0)
    (bind _asbp_first_person_character (Utilities|Casting|CastToBP_FirstPersonCharacter (Game|GetPlayerCharacter 0)))
    (Variables|/Game/FirstPerson/Blueprints/BP_FirstPersonCharacter.BP_FirstPersonCharacter_C|SetisBossDead _asbp_first_person_character true)
    (Actor|DestroyActor)))

(fn ConstructionScript)

(fn HitbyBullet
  (params (BulletDamage :type Integer))
  (bind _output_get (Variables|Default|SetBossHealth (- (Variables|Default|GetBossHealth) BulletDamage)))
  (Development|PrintString (Utilities|String|ToString(Integer) _output_get))
  (if (<= _output_get 0)
    (Actor|DestroyActor)
    (bind _asbp_first_person_character (Utilities|Casting|CastToBP_FirstPersonCharacter (Game|Player|GetPlayerPawn 0)))
    (Default|WinGame _asbp_first_person_character)))