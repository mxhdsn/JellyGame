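; BP_JellyGun is a jelly gun pickup that equips the first-person character.
; On pickup, it reveals the character's own JellyGun component, sets IsGunEquipped and destroys itself.
; Its Fire function line-traces forward from the Arrow with persistent debug drawing and places a decal aligned to the hit normal.
; A projectile spawn with muzzle flash toggling is left unconnected, and the Niagara flash stays paused from BeginPlay.
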(event OnPickUp(TP_PickUp)
  (params (PickUpCharacter :type Jelly%20Game%20Character%20Object%20Reference))
  (bind _asbp_first_person_character (Utilities|Casting|CastToBP_FirstPersonCharacter PickUpCharacter))
  (bind _output_get (Variables|Default|SetCharacterCast _asbp_first_person_character))
  (Rendering|SetVisibility (Variables|/Game/FirstPerson/Blueprints/BP_FirstPersonCharacter.BP_FirstPersonCharacter_C|GetJellyGun _output_get) true false)
  (Variables|/Script/JellyGame.JellyGameCharacter|SetIsGunEquipped _output_get true)
  (Actor|DestroyActor))

(event EventBeginPlay
  (Class|NiagaraComponent|SetPaused (Variables|Default|GetNS_MuzzleFlash) true))

(fn ConstructionScript)

(fn Fire
  (bind _arrow (Variables|Default|GetArrow))
  (bind _returnvalue (Transformation|GetWorldLocation _arrow))
  (bind (_outhit _returnvalue_2) (Collision|LineTraceByChannel _returnvalue (+ _returnvalue (* (Math|Vector|GetForwardVector _arrow) 5e+03)) "TraceTypeQuery1" false 0 "Persistent"))
  (if _returnvalue_2
    (Rendering|Decal|SpawnDecalatLocation 0 "20.000000,20.000000,20.000000" (.Location (Collision|BreakHitResult _outhit)) (Math|Rotator|FindLookatRotation (.Location (Collision|BreakHitResult _outhit)) (+ (.Location (Collision|BreakHitResult _outhit)) (.Normal (Collision|BreakHitResult _outhit)))) 0.0)
    (return)))